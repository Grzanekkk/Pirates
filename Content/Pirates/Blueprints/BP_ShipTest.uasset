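; BP_ShipTest is a test ship Blueprint with debug handlers for collision and water detection, none of which is wired to run.
; Two custom events print the component name on hit and overlap, but the nodes binding them to MainMesh are disconnected.
; A loop printing the Buoyancy component's current water bodies is also disconnected.
; BeginPlay, Tick, ActorBeginOverlap and the construction script are empty.
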(event `self.ReceiveBeginPlay`)

(event `CustomEvent_0`
  (params (OverlappedComponent :type "PrimitiveComponent Object Reference") (OtherActor :type "Actor Object Reference") (OtherComp :type "PrimitiveComponent Object Reference") (OtherBodyIndex :type Integer) (bFromSweep :type Boolean) (SweepResult :type "HitResult Structure (by ref)"))
  (`KismetSystemLibrary.PrintString` (`KismetSystemLibrary.GetDisplayName` OverlappedComponent)))

(event `CustomEvent`
  (params (HitComponent :type "PrimitiveComponent Object Reference") (OtherActor :type "Actor Object Reference") (OtherComp :type "PrimitiveComponent Object Reference") (NormalImpulse :type "Vector Structure") (Hit :type "HitResult Structure (by ref)"))
  (`KismetSystemLibrary.PrintString` (`KismetSystemLibrary.GetDisplayName` HitComponent)))

(event `self.ReceiveActorBeginOverlap`
  (params (OtherActor :type "Actor Object Reference")))

(event `self.ReceiveTick`
  (params (DeltaSeconds :type "Float (single-precision)")))

(fn `UserConstructionScript`)