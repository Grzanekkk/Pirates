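; BP_Sail is a ship sail part whose fabric can be set to a given length.
; RaisSail clamps the requested length to the sail's limits, stores it as SailLength, applies it as the SailFabric X scale and prints it for debugging.
; GetSailDownPrecentage returns SailLength as a fraction of the maximum length, not on a 0-100 scale despite its name.
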(fn `Get Sail Down Precentage`
  (returns (SailsDownPercentage :type "Float (double-precision)"))
  (return (/ (* (`self.SailLength`) (/ 100.0 (`self.MaxSailLength`))) 100.0)))

(fn `RaisSail`
  (params (Length :type "Float (double-precision)"))
  (bind _returnvalue (`KismetMathLibrary.FClamp` Length (`self.MinSailLength`) (`self.MaxSailLength`)))
  (bind (_relativescale3d_x _relativescale3d_y _relativescale3d_z) (`KismetMathLibrary.BreakVector` (`SceneComponent.RelativeScale3D` (`self.SailFabric`))))
  (set `self.SailLength` _returnvalue)
  (`SceneComponent.SetRelativeScale3D` (`self.SailFabric`) (`KismetMathLibrary.MakeVector` _returnvalue _relativescale3d_y _relativescale3d_z))
  (`KismetSystemLibrary.PrintString` (`KismetStringLibrary.Conv_DoubleToString` _returnvalue) true true (struct :`G` 0.66 :`B` 1.0 :`A` 1.0) 0.0))

(fn `UserConstructionScript`)