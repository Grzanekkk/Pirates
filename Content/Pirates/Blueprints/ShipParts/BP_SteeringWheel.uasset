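; BP_SteeringWheel is a ship's steering wheel part that turns the ship according to how far the wheel is rotated.
; Control input adds to the stored wheel value through TurnWheel, which ignores any step that would leave the range of ±180 degrees and pitches the MainShaft component to show the turn.
; Every tick, the accumulated value is passed to the Ship's TurnShip while that reference is valid.
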(event `self.ReceiveTick`
  (params (DeltaSeconds :type "Float (single-precision)"))
  (bind _ship (`self.Ship`))
  (`/Engine/EditorBlueprintResources/StandardMacros.IsValid` _ship
    (:`Is Valid`
      (`/Game/Pirates/Blueprints/BP_ShipTest.TurnShip` _ship (`self.WheelTurnValue`)))))

(event `self.AddControllValueBP`
  (params (ControllDirection :type "Float (single-precision)"))
  (`self.Turn Wheel` ControllDirection))

(fn `Turn Wheel`
  (params (TurnValue :type "Float (double-precision)"))
  (bind _returnvalue (+ TurnValue (`self.WheelTurnValue`)))
  (`|ExecutionSequence`
    (:`then_0`
      (if (and (<= _returnvalue 180.0) (>= _returnvalue -180.0))
        (set `self.WheelTurnValue` _returnvalue)
        (`SceneComponent.K2_SetRelativeRotation` (`self.MainShaft`) (`KismetMathLibrary.MakeRotator` 0.0 _returnvalue 90.0) false false)))))

(fn `UserConstructionScript`)