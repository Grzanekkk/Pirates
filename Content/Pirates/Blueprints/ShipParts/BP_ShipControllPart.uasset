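; Interactable ship control part that lets a pirate character take over the steering wheel.
; Interact sets the STEERINGWHEEL state, flags the part as in use, activates PartCamera and blends the player's view to the part.
; A timer matching the blend time then moves the character to the PlayerLocation component and aligns control rotation with it.
; UnInteract restores WALK, clears the flag and blends the view back to the character.
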(event `PirateInteractionInterface.Interact`
  (params (Instigator :type "Pawn Object Reference"))
  (bind _aspirate_character_base (cast `PirateCharacterBase` Instigator))
  (`PirateCharacterBase.SetPlayerState` _aspirate_character_base "STEERING_WHEEL")
  (set `self.IsPlayerUsingPart` true)
  (`ActorComponent.Activate` (`self.PartCamera`) false)
  (bind _asplayer_controller (cast `PlayerController` (`Pawn.GetController` _aspirate_character_base)))
  (`PlayerController.SetViewTargetWithBlend` _asplayer_controller self 0.5 "VTBlend_Linear" 0.0 false)
  (`KismetSystemLibrary.K2_SetTimerDelegate` (delegate `MovePlayerCharacterToWheel`) 0.5))

(event `MovePlayerCharacterToWheel`
  (bind _playerlocation (`self.PlayerLocation`))
  (`self.K2_SetActorTransform` (stale `PirateInteractionInterface.Interact` _aspirate_character_base) (`KismetMathLibrary.MakeTransform` (`SceneComponent.K2_GetComponentLocation` _playerlocation)) false false)
  (`Controller.SetControlRotation` (`Pawn.GetController` (stale `PirateInteractionInterface.Interact` _aspirate_character_base)) (`SceneComponent.K2_GetComponentRotation` _playerlocation)))

(event `PirateInteractionInterface.UnInteract`
  (params (Instigator :type "Pawn Object Reference"))
  (bind _aspirate_character_base (cast `PirateCharacterBase` Instigator))
  (`PirateCharacterBase.SetPlayerState` _aspirate_character_base "WALK")
  (set `self.IsPlayerUsingPart` false)
  (`PlayerController.SetViewTargetWithBlend` (cast `PlayerController` (`Pawn.GetController` _aspirate_character_base) :!pure true) _aspirate_character_base 0.5 "VTBlend_Linear" 0.0 false))

(fn `UserConstructionScript`)